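; Game mode that sets up audio at play start and switches the music state with the player's alert status.
; BeginPlay caps FPS at 60 by console command, reapplies music and SFX volumes from RSGameInstance, and caches the player controller's Music component.
; PlayerStatusChanged toggles the CurrentState integer parameter on both GameMusicCue and that Music between calm and alerted, based on whether AlertedNum is above zero.
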(event EventBeginPlay
  (Development|ExecuteConsoleCommand "t.maxfps 60" 0)
  (bind _asrsgame_instance (Utilities|Casting|CastToRSGameInstance (Game|GetGameInstance)))
  (bind _asbp_rsplayer_controller (Utilities|Casting|CastToBP_RSPlayerController (Game|GetPlayerController 0))
    (:then
      (Variables|Default|SetMusic (Variables|/Game/Blueprints/Player/BP_RSPlayerController.BP_RSPlayerController_C|GetMusic _asbp_rsplayer_controller)))
    (:CastFailed
      _))
  (Class|RSGameInstance|SetMusicVolume _asrsgame_instance (Class|RSGameInstance|GetMusicVolume _asrsgame_instance))
  (Class|RSGameInstance|SetSfxVolume _asrsgame_instance (Class|RSGameInstance|GetSfxVolume _asrsgame_instance))
  (Effects|Components|ParticleSystem|SetIntParameter (Variables|Default|Getgame_music_cue) "CurrentState" 0)
  (Utilities|IsValid (Variables|Default|GetMusic)
    (:Is%20Valid
      (Effects|Components|ParticleSystem|SetIntParameter (Variables|Default|GetMusic) "CurrentState" 0))))

(event EventTick
  (params (DeltaSeconds :type Float%20%28single-precision%29)))

(event EventPlayerStatusChanged
  (params (SpottedNum :type Integer) (AlertedNum :type Integer))
  (bind _music (Variables|Default|GetMusic))
  (if (> AlertedNum 0)
    (Effects|Components|ParticleSystem|SetIntParameter (Variables|Default|Getgame_music_cue) "CurrentState" 1)
    (Utilities|IsValid _music
      (:Is%20Valid
        (Effects|Components|ParticleSystem|SetIntParameter _music "CurrentState" 1)))
    (else
      (Effects|Components|ParticleSystem|SetIntParameter (Variables|Default|Getgame_music_cue) "CurrentState" 0)
      (Utilities|IsValid _music
        (:Is%20Valid
          (Effects|Components|ParticleSystem|SetIntParameter _music "CurrentState" 0))))))

(fn ConstructionScript)