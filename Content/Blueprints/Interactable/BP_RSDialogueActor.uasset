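; Trigger actor that starts dialogue when a BP_RSBaseCharacter overlaps it, then destroys itself.
; The overlap calls InitializeDialogue on the character and disables the box's collision, making it one-shot.
; Its own DataTable-driven widget path (CreateDialogue, GetDialogueLine) is never called here, and the row filter by nickname and conversation ID is disconnected.
; GetDialogueLine also adds empty strings for speaker and phrase.
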(event EventBeginPlay)

(event Collision|EventActorBeginOverlap
  (params (OtherActor :type Actor%20Object%20Reference))
  (bind _asbp_rsbase_character (Utilities|Casting|CastToBP_RSBaseCharacter OtherActor))
  (Default|InitializeDialogue _asbp_rsbase_character)
  (Collision|SetCollisionResponsetoAllChannels (Variables|Default|GetBox) "ECR_Ignore")
  (Actor|DestroyActor))

(event EventTick
  (params (DeltaSeconds :type Float%20%28single-precision%29)))

(fn ConstructionScript)

(fn CreateDialogue
  (Utilities|IsValid (Variables|Default|GetDialogueWidget)
    (:Is%20Valid
      (bind (_speaker _prasetext _icon) (CallFunction|GetDialogueLine))
      (Variables|/Game/Blueprints/Tutorial/WBP_Dialogue.WBP_Dialogue_C|SetSpeakerNicknameText (Variables|Default|GetDialogueWidget) _speaker)
      (Variables|/Game/Blueprints/Tutorial/WBP_Dialogue.WBP_Dialogue_C|SetPhraseText (Variables|Default|GetDialogueWidget) _prasetext)
      (Variables|/Game/Blueprints/Tutorial/WBP_Dialogue.WBP_Dialogue_C|SetSpeakerIcon (Variables|Default|GetDialogueWidget) _icon))
    (:Is%20Not%20Valid
      (bind _returnvalue (UserInterface|CreateWidget "/Game/Blueprints/Tutorial/WBP_Dialogue.WBP_Dialogue_C" (Game|GetPlayerController 0)))
      (bind _output_get (Variables|Default|SetDialogueWidget _returnvalue))
      (UserInterface|Viewport|AddtoViewport _output_get 0)
      (bind (_speaker_2 _prasetext_2 _icon_2) (CallFunction|GetDialogueLine))
      (Variables|/Game/Blueprints/Tutorial/WBP_Dialogue.WBP_Dialogue_C|SetSpeakerNicknameText (Variables|Default|GetDialogueWidget) _speaker_2)
      (Variables|/Game/Blueprints/Tutorial/WBP_Dialogue.WBP_Dialogue_C|SetPhraseText (Variables|Default|GetDialogueWidget) _prasetext_2)
      (Variables|/Game/Blueprints/Tutorial/WBP_Dialogue.WBP_Dialogue_C|SetSpeakerIcon (Variables|Default|GetDialogueWidget) _icon_2))))

(fn GetDialogueLine
  (bind _returnedlines (LocalVariables|GetReturnedLines))
  (for _array_element (Variables|Default|GetDialogueRowNames)
    (bind _returnvalue (Utilities|GetDataTableRow "/Game/Blueprints/Tutorial/DialogueDataTable.DialogueDataTable" _array_element)
      (:then
        (if (== (.DialogueLine (Utilities|Struct|BreakBP_DialogueDataStructure _returnvalue)) (Variables|Default|GetLineCounter))
          (Utilities|Array|Add (LocalVariables|GetReturnedLines) "")
          (Utilities|Array|Add (LocalVariables|GetReturnedNickname) "")
          (LocalVariables|SetAvatarIcon (.AvaratIcon (Utilities|Struct|BreakBP_DialogueDataStructure _returnvalue)))))))
  (if (== (Utilities|Array|Length _returnedlines) 1)
    (return (Utilities|Array|Get(acopy) (LocalVariables|GetReturnedNickname)) (Utilities|Array|Get(acopy) _returnedlines) (LocalVariables|GetAvatarIcon))
    (else
      (Widget|RemovefromParent (Variables|Default|GetDialogueWidget))
      (Variables|Default|SetDialogueWidget 0)
      (Variables|Default|SetLineCounter 0))))