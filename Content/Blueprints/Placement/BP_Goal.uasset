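; Goal trigger actor that shows the credits and saves the end-game state when its box is overlapped.
; The overlap reuses or creates the head-up widget and plays its ShowCredits animation at reduced speed, without filtering the overlapping actor.
; Animation completion and the player controller's OnQuit event share one path that removes the widget and calls SaveEndGameState on the game instance.
; The menu level load is left unconnected.
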(event OnComponentBeginOverlap(Box)
  (params (OverlappedComponent :type Primitive%20Component%20Object%20Reference) (OtherActor :type Actor%20Object%20Reference) (OtherComp :type Primitive%20Component%20Object%20Reference) (OtherBodyIndex :type Integer) (bFromSweep :type Boolean) (SweepResult :type Hit%20Result%20Structure%20%28by%20ref%29))
  (Utilities|IsValid (Variables|Default|GetHeadUpWidget)
    (:Is%20Valid
      (|PlayAnimationTimeRange (Variables|Default|GetHeadUpWidget) (Variables|/Game/Blueprints/Menu/UI/WBP_HeadUpWidget.WBP_HeadUpWidget_C|GetShowCredits (Variables|Default|GetHeadUpWidget)) 0.0 0.0 1 "Forward" 0.1
        (:Finished
          _)))
    (:Is%20Not%20Valid
      (bind _returnvalue (UserInterface|CreateWidget "/Game/Blueprints/Menu/UI/WBP_HeadUpWidget.WBP_HeadUpWidget_C" (Game|GetPlayerController 0)))
      (bind _output_get (Variables|Default|SetHeadUpWidget _returnvalue))
      (UserInterface|Viewport|AddtoViewport _output_get 0)
      (|PlayAnimationTimeRange (Variables|Default|GetHeadUpWidget) (Variables|/Game/Blueprints/Menu/UI/WBP_HeadUpWidget.WBP_HeadUpWidget_C|GetShowCredits (Variables|Default|GetHeadUpWidget)) 0.0 0.0 1 "Forward" 0.1
        (:Finished
          _))))
  (Widget|RemovefromParent (Variables|Default|GetHeadUpWidget))
  (Variables|Default|SetHeadUpWidget 0)
  (bind _asrsgame_instance (Utilities|Casting|CastToRSGameInstance (Game|GetGameInstance)))
  (Class|RSGameInstance|SaveEndGameState _asrsgame_instance))

(event Custom|CustomEvent_1
  (Widget|RemovefromParent (Variables|Default|GetHeadUpWidget))
  (Variables|Default|SetHeadUpWidget 0)
  (bind _asrsgame_instance (Utilities|Casting|CastToRSGameInstance (Game|GetGameInstance)))
  (Class|RSGameInstance|SaveEndGameState _asrsgame_instance))

(event EventBeginPlay
  (bind _asbp_rsplayer_controller (Utilities|Casting|CastToBP_RSPlayerController (Game|GetPlayerController 0)))
  (EventDispatchers|BindEventtoOnQuit _asbp_rsplayer_controller (delegate Custom|CustomEvent_1)))

(event Collision|EventActorBeginOverlap
  (params (OtherActor :type Actor%20Object%20Reference)))

(event EventTick
  (params (DeltaSeconds :type Float%20%28single-precision%29)))

(fn ConstructionScript)