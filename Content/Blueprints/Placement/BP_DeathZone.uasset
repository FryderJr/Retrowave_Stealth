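; BP_DeathZone is a placeable kill volume that ends the life of any BP_RSBaseCharacter that overlaps it.
; On overlap it disables that character's input through player controller 0, flags it as killed, sets a two-second lifespan and hides its mesh.
; It spawns the Pixelazation Niagara system at the mesh's transform and feeds it that skeletal mesh as the particle source for a dissolve-style death effect.
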(event EventBeginPlay)

(event Collision|EventActorBeginOverlap
  (params (OtherActor :type Actor%20Object%20Reference))
  (bind _asbp_rsbase_character (Utilities|Casting|CastToBP_RSBaseCharacter OtherActor))
  (Input|DisableInput _asbp_rsbase_character (Game|GetPlayerController 0))
  (Variables|/Game/Blueprints/Player/BP_RSBaseCharacter.BP_RSBaseCharacter_C|SetKilled _asbp_rsbase_character true)
  (Actor|SetLifeSpan _asbp_rsbase_character 2.0)
  (Rendering|SetVisibility (Variables|/Script/Engine.Character|GetMesh _asbp_rsbase_character) false false)
  (bind _returnvalue (Niagara|SpawnSystematLocation "/Game/VFX/Pixelazation.Pixelazation" (Transformation|GetWorldLocation (Variables|/Script/Engine.Character|GetMesh _asbp_rsbase_character)) (Transformation|GetWorldRotation (Variables|/Script/Engine.Character|GetMesh _asbp_rsbase_character))))
  (Class|NiagaraFunctionLibrary|OverrideSystemUserVariableSkeletalMeshComponent _returnvalue "User.SM_Source" (Variables|/Script/Engine.Character|GetMesh _asbp_rsbase_character)))

(event EventTick
  (params (DeltaSeconds :type Float%20%28single-precision%29)))

(fn ConstructionScript)