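; Player character Blueprint with a material-driven spawn effect, enemy-triggered death and dialogue input.
; On BeginPlay it caps FPS and moves FollowUp along a spline, feeding a disintegration parameter collection; Tick publishes player position to another.
; An enemy entering the sphere with clear line of sight triggers disintegration, then destruction leaves a replacement camera and loads the last checkpoint.
; E/Q and InitializeDialogue fire dialogue calls; footstep logic is unconnected.
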(event OnComponentBeginOverlap(Sphere)
  (params (OverlappedComponent :type Primitive%20Component%20Object%20Reference) (OtherActor :type Actor%20Object%20Reference) (OtherComp :type Primitive%20Component%20Object%20Reference) (OtherBodyIndex :type Integer) (bFromSweep :type Boolean) (SweepResult :type Hit%20Result%20Structure%20%28by%20ref%29))
  (bind _asbp_enemy (Utilities|Casting|CastToBP_Enemy OtherActor))
  (bind _returnvalue (Collision|LineTraceByChannel (Transformation|GetActorLocation) (Transformation|GetActorLocation _asbp_enemy) "TraceTypeQuery1" false (Utilities|Array|MakeArray _asbp_enemy self) "None"))
  (if (not _returnvalue)
    (Collision|SetCollisionResponsetoAllChannels (Variables|Default|GetSphere) "ECR_Ignore")
    (Input|DisableInput (Game|GetPlayerController 0))
    (Audio|PlaySoundatLocation "/Game/Audio/SCue_death.SCue_death" (Transformation|GetActorLocation) "0, 0, 0" 1.0 1.0 0.0 0 0 0)
    (Class|RSBaseCharacter|SetKilled true)
    (bind _add_track (Timeline|Animate PlayFromStart)
      (:Update
        (Rendering|Material|SetScalarParameterValue "/Game/Dev/MPC_Disintegration.MPC_Disintegration" "add" _add_track :!class /Script/Engine.KismetMaterialLibrary)
        (Rendering|Material|SetVectorParameterValue "/Game/Dev/MPC_Disintegration.MPC_Disintegration" "location" (Utilities|Struct|MakeLinearColor (.X (Math|Vector|BreakVector (Transformation|GetActorLocation _asbp_enemy))) (.Y (Math|Vector|BreakVector (Transformation|GetActorLocation _asbp_enemy))) (.Z (Math|Vector|BreakVector (Transformation|GetActorLocation _asbp_enemy))) 1.0) :!class /Script/Engine.KismetMaterialLibrary))
      (:Finished
        (Actor|SetLifeSpan 0.2)))))

(event Custom|InitializeDialogue
  (bind _outactors (Actor|GetAllActorswithInterface "/Game/Blueprints/Tutorial/BP_DialogueInterface.BP_DialogueInterface_C"))
  (for _array_element _outactors
    (if (Collision|IsOverlappingActor _array_element self :!class /Script/Engine.Actor)
      (Default|CallOnNewDialogue true)
      (Default|CallOnNewPhrase)
      (else
        (Default|CallOnNewDialogue false)))))

(event EventBeginPlay
  (bind _followup (Variables|Default|GetFollowUp))
  (bind _spline (Variables|Default|GetSpline))
  (bind _returnvalue (Transformation|GetWorldLocation _followup))
  (Utilities|FlowControl|Sequence
    (:then_0
      (Development|ExecuteConsoleCommand "t.maxfps 60" 0))
    (:then_1
      (Rendering|SetVisibility _followup true true)
      (bind (_direction _add_track _substract_track _rotate_track) (Timeline|Timeline_2 PlayFromStart)
        (:Update
          (Rendering|Material|SetScalarParameterValue "/Game/Dev/MPC_Disintegration.MPC_Disintegration" "add" _substract_track :!class /Script/Engine.KismetMaterialLibrary)
          (Rendering|Material|SetVectorParameterValue "/Game/Dev/MPC_Disintegration.MPC_Disintegration" "location" (Utilities|Struct|MakeLinearColor (.x _returnvalue) (.y _returnvalue) (.z _returnvalue) 1.0) :!class /Script/Engine.KismetMaterialLibrary)
          (Transformation|SetRelativeLocation (Variables|Default|GetFollowUp) (Spline|GetLocationatDistanceAlongSpline _spline (Math|Float|Lerp 0.0 (Spline|GetSplineLength _spline) _rotate_track) "Local") false false))
        (:Finished
          (Rendering|SetVisibility (Variables|Default|GetFollowUp) false true)
          (Rendering|Material|SetScalarParameterValue "/Game/Dev/MPC_Disintegration.MPC_Disintegration" "add" -3.0 :!class /Script/Engine.KismetMaterialLibrary))))))

(event Collision|EventActorBeginOverlap
  (params (OtherActor :type Actor%20Object%20Reference)))

(event EventTick
  (params (DeltaSeconds :type Float%20%28single-precision%29))
  (bind _returnvalue (Transformation|GetActorLocation))
  (Rendering|Material|SetVectorParameterValue "/Game/Dev/MPC_Test.MPC_Test" "Position" (Utilities|Struct|MakeLinearColor (.x _returnvalue) (.y _returnvalue) (.z _returnvalue) 1.0) :!class /Script/Engine.KismetMaterialLibrary))

(event EventDestroyed
  (bind _returnvalue (Game|GetPlayerController 0))
  (bind _returnvalue_2 (Game|SpawnActorfromClass "/Script/Engine.CameraActor" (Transformation|GetWorldTransform (Variables|Default|GetFollowCamera)) "Undefined" 0 0))
  (Camera|SetFieldOfView (Variables|/Script/Engine.CameraActor|GetCameraComponent _returnvalue_2) 9e+01)
  (Game|Player|SetViewTargetwithBlend _returnvalue _returnvalue_2 0.0 "VTBlend_PreBlended" 0.0 true)
  (if (Variables|Default|GetbKilled)
    (bind _asbp_rsplayer_controller (Utilities|Casting|CastToBP_RSPlayerController _returnvalue))
    (Default|LoadLastCheckpoint _asbp_rsplayer_controller)))

(event Input|KeyboardEvents|E
  (params (Key :type Key%20Structure :default "None"))
  (:Pressed
    (Default|CallOnNewPhrase)))

(event Input|KeyboardEvents|Q
  (params (Key :type Key%20Structure :default "None"))
  (:Pressed
    (Default|CallOnQuitDialogue)))

(fn ConstructionScript)