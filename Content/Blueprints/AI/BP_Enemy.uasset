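; BP_Enemy is an enemy actor that sweeps searchlight-style Niagara rays from a mesh socket along a spline.
; A looping timer advances spline time and feeds each of three Niagara components a start and end point, each offset by a delay to form a trailing sweep.
; Visibility traces cut each ray at blocking hits.
; A one-second check pauses the sweep unless the BP_RSBaseCharacter is within range.
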(event Custom|CustomEvent_0
  (bind _searchtimer (Variables|Default|GetSearchTimer))
  (bind _returnvalue (Actor|GetActorOfClass "/Game/Blueprints/Player/BP_RSBaseCharacter.BP_RSBaseCharacter_C"))
  (Utilities|IsValid _returnvalue
    (:Is%20Valid
      (if (< (Math|Vector|Distance(Vector) (Transformation|GetActorLocation) (Transformation|GetActorLocation _returnvalue)) 4e+03)
        (Utilities|Time|UnpauseTimerbyHandle _searchtimer)
        (else
          (Utilities|Time|PauseTimerbyHandle _searchtimer))))))

(event Custom|GetSplineLocation
  (if (> (+ (Variables|Default|GetSplineTime) 0.05) (+ (Variables|/Script/Engine.SplineComponent|GetDuration (Variables|Default|GetSpline)) (* (Utilities|Array|Length (Variables|Default|GetNiagaraArray)) (Variables|Default|GetDelay))))
    (Variables|Default|SetSplineTime 0.0)
    (else
      (Variables|Default|SetSplineTime (+ (Variables|Default|GetSplineTime) 0.05))))
  (for (_array_element _array_index) (Variables|Default|GetNiagaraArray)
    (bind (_startraylocation _endraylocation) (CallFunction|GetSearhingRayCoords (* _array_index (Variables|Default|GetDelay))))
    (Niagara|SetNiagaraVariable(Vector3) _array_element "USER.RayStart" _startraylocation)
    (Niagara|SetNiagaraVariable(Vector3) _array_element "USER.RayEnd" _endraylocation)))

(event EventBeginPlay
  (Utilities|FlowControl|Sequence
    (:then_0
      (bind _returnvalue (AddComponent|AddNiagaraComponent false))
      (Utilities|Array|Add (Variables|Default|GetNiagaraArray) _returnvalue)
      (bind _returnvalue_2 (AddComponent|AddNiagaraComponent false))
      (Utilities|Array|Add (Variables|Default|GetNiagaraArray) _returnvalue_2)
      (bind _returnvalue_3 (AddComponent|AddNiagaraComponent false))
      (Utilities|Array|Add (Variables|Default|GetNiagaraArray) _returnvalue_3))
    (:then_1
      (bind _returnvalue_4 (Utilities|Time|SetTimerbyEvent (delegate Custom|GetSplineLocation) 0.05 true))
      (Variables|Default|SetSearchTimer _returnvalue_4))
    (:then_2
      (Utilities|Time|SetTimerbyEvent (delegate Custom|CustomEvent_0) 1.0 true))))

(event Collision|EventActorBeginOverlap
  (params (OtherActor :type Actor%20Object%20Reference)))

(event EventTick
  (params (DeltaSeconds :type Float%20%28single-precision%29)))

(event EventEndPlay
  (params (EndPlayReason :type EEndPlayReason%20Enum :default "Destroyed")))

(fn ConstructionScript)

(fn GetSearhingRayCoords
  (params (Delay :type Float%20%28single-precision%29))
  (bind _mesh (Variables|Character|GetMesh))
  (bind _spline (Variables|Default|GetSpline))
  (bind _splinetime (Variables|Default|GetSplineTime))
  (bind _returnvalue (Transformation|GetSocketLocation _mesh "SearchRaySocket"))
  (if (< _splinetime Delay)
    (LocalVariables|SetLocalTime 0.0)
    (else
      (LocalVariables|SetLocalTime (- _splinetime Delay))))
  (bind _outhit (Collision|LineTraceByChannel _returnvalue (Spline|GetLocationatTime _spline (Math|Float|Clamp(Float) (LocalVariables|GetLocalTime) 0.0 (Variables|/Script/Engine.SplineComponent|GetDuration _spline)) "World" false) "TraceTypeQuery1" false 0 "None"))
  (if (.bblockinghit _outhit)
    (return _returnvalue (.location _outhit))
    (else
      (return _returnvalue (Spline|GetLocationatTime _spline (Math|Float|Clamp(Float) (LocalVariables|GetLocalTime) 0.0 (Variables|/Script/Engine.SplineComponent|GetDuration _spline)) "World" false)))))