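; Behavior tree task that returns an enemy to an unalerted state after the player escapes its sight.
; It resets the enemy's audio state parameter, turns its spotlight blue and removes it from the game mode's alerted-by and spotted-by records.
; It then makes AI perception forget all stimuli and clears the player blackboard key, succeeding only when the owner is a BP_EnemyController.
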(event EventReceiveExecuteAI
  (params (OwnerController :type AI%20Controller%20Object%20Reference) (ControlledPawn :type Pawn%20Object%20Reference))
  (Utilities|FlowControl|Sequence
    (:then_0
      (bind _asbp_enemy (Utilities|Casting|CastToBP_Enemy ControlledPawn))
      (Effects|Components|ParticleSystem|SetIntParameter (Variables|/Game/Blueprints/AI/BP_Enemy.BP_Enemy_C|GetAudio _asbp_enemy) "Enemy_state" 0)
      (Rendering|Components|Light|SetLightColor (Variables|/Game/Blueprints/AI/BP_Enemy.BP_Enemy_C|GetSpotLight _asbp_enemy) "(R=0.000000,G=0.000000,B=20.000000,A=1.000000)" true)
      (bind _asbp_rsgame_mode (Utilities|Casting|CastToBP_RSGameMode (Game|GetGameMode)))
      (Class|RSGameMode|DeleteAlertedby _asbp_rsgame_mode _asbp_enemy)
      (Class|RSGameMode|DeleteSpottedby _asbp_rsgame_mode _asbp_enemy))
    (:then_1
      (Class|AIPerceptionComponent|ForgetAll (Class|AIController|GetAIPerceptionComponent OwnerController))
      (Utilities|Casting|CastToBP_EnemyController OwnerController
        (:then
          (Class|BTFunctionLibrary|SetBlackboardValueasObject (Variables|Default|GetPlayerBlackboardKey))
          (AI|BehaviorTree|FinishExecute true))
        (:CastFailed
          (AI|BehaviorTree|FinishExecute false))))))