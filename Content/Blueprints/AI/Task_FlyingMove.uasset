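; Behavior tree task that flies an AI Character toward a blackboard Destination, either an Actor or a vector.
; Each tick it adds movement input along the 3D look-at direction, aimed slightly above the target, and lerps the character's rotation in yaw only.
; It succeeds within Distance of the target or after a short timeout, so timing out also counts as success.
; It fails if the pawn is not a Character.
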(event EventReceiveTickAI
  (params (OwnerController :type AI%20Controller%20Object%20Reference) (ControlledPawn :type Pawn%20Object%20Reference) (DeltaSeconds :type Float%20%28single-precision%29))
  (bind _destination (Variables|Default|GetDestination))
  (bind _returnvalue (Class|BTFunctionLibrary|GetBlackboardValueasObject _destination))
  (bind _output_get (Variables|Default|SetCurrentTime (+ DeltaSeconds (Variables|Default|GetCurrentTime))))
  (if (> _output_get 1.5)
    (AI|BehaviorTree|FinishExecute true)
    (else
      (Utilities|IsValid _returnvalue
        (:Is%20Valid
          (bind _asactor (Utilities|Casting|CastToActor _returnvalue))
          (Variables|Default|SetLocation (Transformation|GetActorLocation _asactor)))
        (:Is%20Not%20Valid
          (Variables|Default|SetLocation (Class|BTFunctionLibrary|GetBlackboardValueasVector (Variables|Default|GetDestination)))))
      (bind _ascharacter (Utilities|Casting|CastToCharacter ControlledPawn)
        (:then
          (if (< (Math|Vector|VectorLength (- (Transformation|GetActorLocation _ascharacter) (Variables|Default|GetLocation))) (Variables|Default|GetDistance))
            (AI|BehaviorTree|FinishExecute true)
            (else
              (Class|PawnMovementComponent|AddInputVector (Pawn|GetMovementComponent _ascharacter) (Math|Rotator|GetRotationXVector (Math|Rotator|MakeRotator 0.0 (.pitch (Math|Rotator|FindLookatRotation (Transformation|GetActorLocation _ascharacter) (+ (Variables|Default|GetLocation) "0, 0,5.000000"))) (.yaw (Math|Rotator|FindLookatRotation (Transformation|GetActorLocation _ascharacter) (+ (Variables|Default|GetLocation) "0, 0,5.000000"))))) false)
              (Transformation|SetActorRotation _ascharacter (Math|Rotator|Lerp(Rotator) (Transformation|GetActorRotation _ascharacter) (Math|Rotator|MakeRotator 0.0 0.0 (.yaw (Math|Rotator|FindLookatRotation (Transformation|GetActorLocation _ascharacter) (+ (Variables|Default|GetLocation) "0, 0,5.000000")))) 0.1 true)))))
        (:CastFailed
          (AI|BehaviorTree|FinishExecute false))))))

(event EventReceiveExecuteAI
  (params (OwnerController :type AI%20Controller%20Object%20Reference) (ControlledPawn :type Pawn%20Object%20Reference))
  (Variables|Default|SetCurrentTime 0.0))