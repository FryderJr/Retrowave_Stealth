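; Behavior tree task that finds a player character known to the AI's perception and stores it in the blackboard.
; It scans the controller's known perceived actors and stops at the first Character with a player controller.
; Despite the asset name, it writes the character object to the Player key rather than a position.
; It finishes with success only if the stored character reference is valid.
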(event EventReceiveExecuteAI
  (params (OwnerController :type AI%20Controller%20Object%20Reference) (ControlledPawn :type Pawn%20Object%20Reference))
  (bind _array_element (Utilities|Array|ForEachLoopwithBreak (Class|AIPerceptionComponent|GetKnownPerceivedActors (Class|AIController|GetAIPerceptionComponent OwnerController)) :!label _label)
    (:LoopBody
      (bind _ascharacter (Utilities|Casting|CastToCharacter _array_element))
      (if (Class|Controller|IsPlayerController (Pawn|GetController _ascharacter))
        (Variables|Default|SetPercievedCharacter _ascharacter)
        (goto _label Break)))
    (:Completed
      (Class|BTFunctionLibrary|SetBlackboardValueasObject (Variables|Default|GetPlayer) (Variables|Default|GetPercievedCharacter))
      (AI|BehaviorTree|FinishExecute (Utilities|IsValid (Variables|Default|GetPercievedCharacter))))))