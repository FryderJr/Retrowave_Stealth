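; Behavior tree task that finds the spline path nearest to the controlled pawn and stores it on the blackboard.
; On execute it scans every BP_Spline actor, measuring from the pawn to the closest point on each spline.
; The nearest actor under the ClosestSplineDistance threshold, which is not reset in the graph, becomes CurrentSpline.
; It writes CurrentSpline to the Path key and always finishes successfully.
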(event EventReceiveExecuteAI
  (params (OwnerController :type AI%20Controller%20Object%20Reference) (ControlledPawn :type Pawn%20Object%20Reference))
  (bind _returnvalue (Transformation|GetActorLocation ControlledPawn))
  (bind _outactors (Actor|GetAllActorsOfClass "/Game/Blueprints/AI/BP_Spline.BP_Spline_C"))
  (for _array_element _outactors
    (if (< (Math|Vector|VectorLength (- (Spline|FindLocationClosesttoWorldLocation (Variables|/Game/Blueprints/AI/BP_Spline.BP_Spline_C|GetSplinePath _array_element) _returnvalue "World") _returnvalue)) (Variables|Default|GetClosestSplineDistance))
      (Variables|Default|SetClosestSplineDistance (Math|Vector|VectorLength (- (Spline|FindLocationClosesttoWorldLocation (Variables|/Game/Blueprints/AI/BP_Spline.BP_Spline_C|GetSplinePath _array_element) _returnvalue "World") _returnvalue)))
      (Variables|Default|SetCurrentSpline _array_element)))
  (Class|BTFunctionLibrary|SetBlackboardValueasObject (Variables|Default|GetPath) (Variables|Default|GetCurrentSpline))
  (AI|BehaviorTree|FinishExecute true))