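; Enemy AI controller that starts the BT_Enemy behavior tree on BeginPlay and maintains player references in its Blackboard.
; SetPlayer writes an actor to a given Blackboard key, and OnPlayerEscaped clears the player key.
; The perception update event and SensedPlayer are empty stubs, so sensing does not feed the Blackboard here, and a debug-sphere draw is left unconnected.
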(event OnTargetPerceptionUpdated(AIPerception)
  (params (Actor :type Actor%20Object%20Reference) (Stimulus :type AI%20Stimulus%20Structure)))

(event Custom|On%20Player%20Escaped
  (AI|Components|Blackboard|SetValueasObject (AI|GetBlackboard 0) (Variables|Default|GetPlayerBlackboardName) 0))

(event EventBeginPlay
  (AI|RunBehaviorTree "/Game/Blueprints/AI/BT_Enemy.BT_Enemy"))

(event EventTick
  (params (DeltaSeconds :type Float%20%28single-precision%29)))

(fn ConstructionScript)

(fn SensedPlayer
  (params (BlackboardKey :type Name) (Stimuli :type AI%20Stimulus%20Structure) (SensedActor :type Actor%20Object%20Reference)))

(fn SetPlayer
  (params (BlackboardKey :type Name) (Actor :type Actor%20Object%20Reference))
  (AI|Components|Blackboard|SetValueasObject (AI|GetBlackboard 0) BlackboardKey Actor))