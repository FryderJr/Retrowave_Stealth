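; Behavior tree task that makes an enemy raise the alarm when alerting others to the player.
; It tints the BP_Enemy spotlight red and sets the game mode audio component's CurrentState parameter to 1.
; It then reports a loud noise at the enemy's location with the player as instigator, failing if no valid player pawn exists.
; An unconnected older approach writes the player into nearby enemies' blackboards directly.
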(event EventReceiveExecuteAI
  (params (OwnerController :type AI%20Controller%20Object%20Reference) (ControlledPawn :type Pawn%20Object%20Reference))
  (bind _returnvalue (Game|Player|GetPlayerPawn 0))
  (Utilities|FlowControl|Sequence
    (:then_0
      (bind _asbp_enemy (Utilities|Casting|CastToBP_Enemy ControlledPawn))
      (Rendering|Components|Light|SetLightColor (Variables|/Game/Blueprints/AI/BP_Enemy.BP_Enemy_C|GetSpotLight _asbp_enemy) "(R=20.000000,G=0.000000,B=0.000000,A=1.000000)" true)
      (bind _asbp_rsgame_mode (Utilities|Casting|CastToBP_RSGameMode (Game|GetGameMode)))
      (Effects|Components|ParticleSystem|SetIntParameter (Actor|GetComponentbyClass _asbp_rsgame_mode "/Script/Engine.AudioComponent") "CurrentState" 1))
    (:then_1
      (Utilities|IsValid _returnvalue
        (:Is%20Valid
          (Class|AISenseHearing|ReportNoiseEvent (Transformation|GetActorLocation ControlledPawn) 5.0 _returnvalue 0.0 "None")
          (AI|BehaviorTree|FinishExecute true))
        (:Is%20Not%20Valid
          (AI|BehaviorTree|FinishExecute false))))))