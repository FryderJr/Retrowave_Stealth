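; Behavior tree decorator that passes when the AI's controlled pawn is very close to the first player's pawn.
; Its AI condition check compares the straight-line distance between the two pawns against a small hard-coded threshold, and fails when no valid player pawn exists.
; The event graph holds only an unused, disconnected copy of the distance test.
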(fn PerformConditionCheckAI
  (params (OwnerController :type AI%20Controller%20Object%20Reference) (ControlledPawn :type Pawn%20Object%20Reference))
  (bind _returnvalue (Game|Player|GetPlayerPawn 0))
  (Utilities|IsValid _returnvalue
    (:Is%20Valid
      (return (< (Math|Vector|VectorLength (- (Transformation|GetActorLocation ControlledPawn) (Transformation|GetActorLocation _returnvalue))) 5e+01)))
    (:Is%20Not%20Valid
      (return false))))