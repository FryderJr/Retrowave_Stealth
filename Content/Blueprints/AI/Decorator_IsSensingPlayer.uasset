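; Behavior Tree decorator that passes when the AI currently senses the player.
; It reads the controller's AI Perception data for the first player's pawn and scans the last sensed stimuli from every sense.
; A stimulus counts only if it is under a second old and lies almost exactly at the player's present location, filtering out stale or displaced detections.
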(fn PerformConditionCheckAI
  (params (OwnerController :type AI%20Controller%20Object%20Reference) (ControlledPawn :type Pawn%20Object%20Reference))
  (bind _returnvalue (Game|Player|GetPlayerPawn 0))
  (bind _info (Class|AIPerceptionComponent|GetActorsPerception (Class|AIController|GetAIPerceptionComponent OwnerController) _returnvalue))
  (bind _array_element (Utilities|Array|ForEachLoopwithBreak (.lastsensedstimuli _info))
    (:LoopBody
      (if (and (< (.age _array_element) 0.75) (< (Math|Vector|VectorLength (- (.stimuluslocation _array_element) (Transformation|GetActorLocation _returnvalue))) 2e+01))
        (return true)))
    (:Completed
      (return false))))