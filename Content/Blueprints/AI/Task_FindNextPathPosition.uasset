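; Behavior tree task that picks the next point for an AI character to head to along a BP_Spline path.
; It advances the PathCovered blackboard distance by the character's max movement speed, then writes that spline location in world space to NextPathPoint.
; When the new distance passes 95% of the spline length, it resets PathCovered to zero and fails.
; It also fails when PathObject is not a BP_Spline.
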(event EventReceiveExecuteAI
  (params (OwnerController :type AI%20Controller%20Object%20Reference) (ControlledPawn :type Pawn%20Object%20Reference))
  (bind _asbp_spline (Utilities|Casting|CastToBP_Spline (AI|BehaviorTree|GetBlackboardValueasActor (Variables|Default|GetPathObject)))
    (:then
      (if (> (/ (+ (Class|BTFunctionLibrary|GetBlackboardValueasFloat (Variables|Default|GetPathCovered)) (Class|MovementComponent|GetMaxSpeed (Pawn|GetMovementComponent (.AsCharacter (Utilities|Casting|CastToCharacter ControlledPawn))))) (Spline|GetSplineLength (Variables|/Game/Blueprints/AI/BP_Spline.BP_Spline_C|GetSplinePath _asbp_spline))) 0.95)
        (Class|BTFunctionLibrary|SetBlackboardValueasFloat (Variables|Default|GetPathCovered) 0.0)
        (AI|BehaviorTree|FinishExecute false)
        (else
          (Class|BTFunctionLibrary|SetBlackboardValueasFloat (Variables|Default|GetPathCovered) (Math|Float|Lerp 0.0 (Spline|GetSplineLength (Variables|/Game/Blueprints/AI/BP_Spline.BP_Spline_C|GetSplinePath _asbp_spline)) (/ (+ (Class|BTFunctionLibrary|GetBlackboardValueasFloat (Variables|Default|GetPathCovered)) (Class|MovementComponent|GetMaxSpeed (Pawn|GetMovementComponent (.AsCharacter (Utilities|Casting|CastToCharacter ControlledPawn))))) (Spline|GetSplineLength (Variables|/Game/Blueprints/AI/BP_Spline.BP_Spline_C|GetSplinePath _asbp_spline)))))
          (AI|BehaviorTree|SetBlackboardValueasVector (Variables|Default|GetNextPathPoint) (Spline|GetLocationatDistanceAlongSpline (Variables|/Game/Blueprints/AI/BP_Spline.BP_Spline_C|GetSplinePath _asbp_spline) (Math|Float|Lerp 0.0 (Spline|GetSplineLength (Variables|/Game/Blueprints/AI/BP_Spline.BP_Spline_C|GetSplinePath _asbp_spline)) (/ (+ (Class|BTFunctionLibrary|GetBlackboardValueasFloat (Variables|Default|GetPathCovered)) (Class|MovementComponent|GetMaxSpeed (Pawn|GetMovementComponent (.AsCharacter (Utilities|Casting|CastToCharacter ControlledPawn))))) (Spline|GetSplineLength (Variables|/Game/Blueprints/AI/BP_Spline.BP_Spline_C|GetSplinePath _asbp_spline)))) "World"))
          (AI|BehaviorTree|FinishExecute true))))
    (:CastFailed
      (AI|BehaviorTree|FinishExecute false))))